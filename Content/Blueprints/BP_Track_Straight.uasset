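; BP_Track_Straight is a straight track tile for an endless vehicle game, exposing its AttachPoint transform through GetAttachTransform.
; A vehicle entering EndTrigger makes the VehicleAdvGameMode add a floor tile, then this tile destroys itself after a short delay.
; A Racer touching DeathFloor triggers its Death.
; The construction script calls SpawnCoins, which adds one child actor at a random point inside the CoinArea box.
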(event OnComponentBeginOverlap(EndTrigger)
  (params (OverlappedComponent :type Primitive%20Component%20Object%20Reference) (OtherActor :type Actor%20Object%20Reference) (OtherComp :type Primitive%20Component%20Object%20Reference) (OtherBodyIndex :type Integer) (bFromSweep :type Boolean) (SweepResult :type Hit%20Result%20Structure%20%28by%20ref%29))
  (Utilities|Casting|CastToWheeledVehicle OtherActor)
  (bind _asvehicle_adv_game_mode (Utilities|Casting|CastToVehicleAdvGameMode (Game|GetGameMode)))
  (Default|AddFloorTile _asvehicle_adv_game_mode)
  (Utilities|FlowControl|Delay 2.0)
  (Actor|DestroyActor))

(event OnComponentBeginOverlap(DeathFloor)
  (params (OverlappedComponent :type Primitive%20Component%20Object%20Reference) (OtherActor :type Actor%20Object%20Reference) (OtherComp :type Primitive%20Component%20Object%20Reference) (OtherBodyIndex :type Integer) (bFromSweep :type Boolean) (SweepResult :type Hit%20Result%20Structure%20%28by%20ref%29))
  (bind _asracer (Utilities|Casting|CastToRacer OtherActor))
  (Default|Death _asracer))

(event EventBeginPlay)

(event Collision|EventActorBeginOverlap
  (params (OtherActor :type Actor%20Object%20Reference)))

(event EventTick
  (params (DeltaSeconds :type Float%20%28single-precision%29)))

(fn ConstructionScript
  (CallFunction|SpawnCoins))

(fn GetAttachTransform
  (return (Transformation|GetWorldTransform (Variables|Default|GetAttachPoint))))

(fn SpawnCoins
  (bind _coinarea (Variables|Default|GetCoinArea))
  (AddComponent|AddChildActorComponent false (Math|Conversions|ToTransform(Vector) (Math|Random|RandomPointinBoundingBox (Variables|/Script/Engine.SceneComponent|GetRelativeLocation _coinarea) (Variables|/Script/Engine.BoxComponent|GetBoxExtent _coinarea)))))